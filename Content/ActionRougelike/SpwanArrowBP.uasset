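; SpwanArrowBP is a turret-like actor that fires magic projectiles toward the player.
; Each tick it rotates to look at the location of its Player reference, which is not assigned in these graphs.
; From BeginPlay, a looping timer spawns a MagicProjectileBP every two seconds at the actor's own location and rotation, so shots follow its current aim.
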(event Custom|SpwanActor
  (Game|SpawnActorfromClass "/Game/ActionRougelike/MagicProjectileBP.MagicProjectileBP_C" (Math|Transform|MakeTransform (Transformation|GetActorLocation) (Transformation|GetActorRotation)) "Undefined" 0 0))

(event EventBeginPlay
  (Utilities|Time|SetTimerbyEvent (delegate Custom|SpwanActor) 2.0 true))

(event Collision|EventActorBeginOverlap
  (params (OtherActor :type Actor%20Object%20Reference)))

(event EventTick
  (params (DeltaSeconds :type Float%20%28single-precision%29))
  (Transformation|SetActorRotation (Math|Rotator|FindLookatRotation (Transformation|GetActorLocation) (Transformation|GetActorLocation (Variables|Default|GetPlayer)))))

(fn ConstructionScript)