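; Explosive barrel actor that explodes on a server-started timer shortly after BeginPlay.
; The authority calls a multicast that fires the RadialForce impulse, prints a debug message, hides the actor and disables collision.
; It then sets a short lifespan instead of destroying immediately, so the multicast reaches clients before the actor is gone.
; The mesh hit event does nothing, and the damage logic is disconnected.
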(event OnComponentHit(StaticMesh)
  (params (HitComponent :type Primitive%20Component%20Object%20Reference) (OtherActor :type Actor%20Object%20Reference) (OtherComp :type Primitive%20Component%20Object%20Reference) (NormalImpulse :type Vector :default "0, 0, 0") (Hit :type Hit%20Result%20Structure%20%28by%20ref%29))
  (Utilities|IsValid OtherActor))

(event Custom|Explode
  (CallFunction|MulticastExplode)
  (Actor|SetLifeSpan 2.0))

(event Custom|MulticastExplode
  (Development|PrintString "EXPLODE!" true true "(R=1.000000,G=0.000000,B=0.060073,A=1.000000)" 1e+01)
  (Class|RadialForceComponent|FireImpulse (Variables|Default|GetRadialForce))
  (Rendering|SetActorHiddenInGame true)
  (Collision|SetActorEnableCollision false))

(event EventBeginPlay
  (if (Ability|HasAuthority)
    (Utilities|Time|SetTimerbyEvent (delegate Custom|Explode) 4.0)))

(fn ConstructionScript)